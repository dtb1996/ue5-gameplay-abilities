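; Actor component that manages equipping and unequipping weapons on its owning Character.
; EquipWeapon spawns the weapon class and snaps it to a mesh socket, replacing any held weapon; requesting the held class again just unequips it.
; Each weapon's config drives the character's anim class, walk speed and rotation mode.
; Unequipping destroys the weapon actor and restores those settings from an unarmed config.
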(event `self.ReceiveBeginPlay`
  (bind _ascharacter (cast `Character` (`self.GetOwner`)))
  (set `self.OwningCharacter` _ascharacter))

(event `EquipWeapon`
  (params (WeaponClass :type "/Game/Weapons/BP_Weapon_Base Class Reference"))
  (bind _charactermovement (`Character.CharacterMovement` (`self.OwningCharacter`)))
  (`self.OwningCharacter`
    (:`then`
      (bind _equippedweapon (`self.EquippedWeapon`)
        (:`then`
          (if (== (`GameplayStatics.GetObjectClass` _equippedweapon) WeaponClass)
            (`self.UnequipWeapon`)
            (else
              (`self.UnequipWeapon`)
              (bind _returnvalue (`|SpawnActorFromClass` WeaponClass (`KismetMathLibrary.MakeTransform` (0.0 0.0 0.0)) "Undefined" "MultiplyWithRoot" null null :!label _label))
              (bind _output_get (set `self.EquippedWeapon` _returnvalue))
              (bind ((`EquippedSocketName_7_1A9E89E7419170AE2760CEAA0411F455` _equippedsocketname) (`AnimClass_10_4668A7DF4AE64FDBC82C0AB587F556CF` _animclass) (`MovementProperties_14_9655A31943DB22F772B0F1804EC24CE1` _movementproperties)) (break `/Game/Weapons/Data/S_WeaponConfig` (`/Game/Weapons/BP_Weapon_Base.WeaponConfig` _output_get)))
              (`Actor.K2_AttachToComponent` _output_get (`Character.Mesh` (`self.OwningCharacter`)) _equippedsocketname "SnapToTarget" "SnapToTarget" "SnapToTarget" true)
              (`SkeletalMeshComponent.SetAnimInstanceClass` (`Character.Mesh` (`self.OwningCharacter`)) _animclass)
              (bind (_maxwalkspeed _orientrotationtomovement _usecontrollerdesiredrotation) (break `/Game/Weapons/Data/S_MovementProperties` _movementproperties))
              (set `CharacterMovementComponent.MaxWalkSpeed` _maxwalkspeed _charactermovement)
              (set `CharacterMovementComponent.bOrientRotationToMovement` _orientrotationtomovement _charactermovement)
              (set `CharacterMovementComponent.bUseControllerDesiredRotation` _usecontrollerdesiredrotation _charactermovement))))
        (:`else`
          (goto _label))))
    (:`else`)))

(event `UnequipWeapon`
  (bind ((`AnimClass_10_4668A7DF4AE64FDBC82C0AB587F556CF` _animclass) (`MovementProperties_14_9655A31943DB22F772B0F1804EC24CE1` _movementproperties)) (break `/Game/Weapons/Data/S_WeaponConfig` (`self.UnarmedWeaponConfig`)))
  (bind _charactermovement (`Character.CharacterMovement` (`self.OwningCharacter`)))
  (bind (_maxwalkspeed _orientrotationtomovement _usecontrollerdesiredrotation) (break `/Game/Weapons/Data/S_MovementProperties` _movementproperties))
  (bind _equippedweapon (`self.EquippedWeapon`)
    (:`then`
      (`Actor.K2_DestroyActor` _equippedweapon)
      (set `self.EquippedWeapon` null)
      (`SkeletalMeshComponent.SetAnimInstanceClass` (`Character.Mesh` (`self.OwningCharacter`)) _animclass)
      (set `CharacterMovementComponent.MaxWalkSpeed` _maxwalkspeed _charactermovement)
      (set `CharacterMovementComponent.bOrientRotationToMovement` _orientrotationtomovement _charactermovement)
      (set `CharacterMovementComponent.bUseControllerDesiredRotation` _usecontrollerdesiredrotation _charactermovement))
    (:`else`)))