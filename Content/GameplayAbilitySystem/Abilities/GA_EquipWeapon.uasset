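; Gameplay ability that switches the avatar's weapon in response to a gameplay event.
; It commits, then, if the avatar has a BP_WeaponsManagerComponent, switches on the first target tag in the event data.
; Staff and axe tags tell the component to equip the matching weapon class, and any other tag unequips.
; The ability ends right after the switch, but has no end call when the component is missing.
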(event `self.K2_ActivateAbilityFromEvent`
  (params (EventData :type "GameplayEventData Structure (by ref)"))
  (bind _returnvalue (`Actor.GetComponentByClass` (`self.GetAvatarActorFromActorInfo`) "/Game/Weapons/BP_WeaponsManagerComponent.BP_WeaponsManagerComponent_C"))
  (`self.K2_CommitAbility`)
  (`/Engine/EditorBlueprintResources/StandardMacros.IsValid` _returnvalue
    (:`Is Valid`
      (`|ExecutionSequence`
        (:`then_0`
          (`|SwitchGameplayTag` (`|GetArrayItem` (`BlueprintGameplayTagLibrary.BreakGameplayTagContainer` (`.TargetTags` (break `GameplayEventData` EventData))))
            (:`Default`
              (`/Game/Weapons/BP_WeaponsManagerComponent.UnequipWeapon` _returnvalue))
            (:`Weapon.Ranged.Staff`
              (`/Game/Weapons/BP_WeaponsManagerComponent.EquipWeapon` _returnvalue "/Game/Weapons/BP_Weapon_Staff.BP_Weapon_Staff_C"))
            (:`Weapon.Melee.Axe`
              (`/Game/Weapons/BP_WeaponsManagerComponent.EquipWeapon` _returnvalue "/Game/Weapons/BP_Weapon_Axe.BP_Weapon_Axe_C"))))
        (:`then_1`
          (`self.K2_EndAbility`))))))